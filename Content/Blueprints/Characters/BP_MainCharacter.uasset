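; Player character Blueprint that handles horizontal look, movement and projectile shooting.
; Move axes feed movement input along forward and right vectors that a ControlRotation helper derives from the camera's full world rotation, including pitch and roll.
; Pressing Fire spawns BP_ProjectileBase using a helper that converts the ShootDirection arrow into a transform, nudged one unit along its forward vector.
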(event Input|ActionEvents|InputActionFire
  (params (Key :type Key%20Structure :default "None"))
  ;[1 0.0191 0] Fire: Using the ShootDirection arrow as a reference, and Input Fire as a trigger, I created a custom function ('GetSceneComponentLocationIntoTransform'), to get the location of shoot direction arrow into Transform and use it to Spawn an Actor, in this case a Projectile class, in order to shoot
  (:Pressed
    (bind _locationtransform (CallFunction|GetSceneComponentLocationIntoTransform (Variables|Default|GetShootDirection)))
    (Game|SpawnActorfromClass "/Game/Blueprints/Projectiles/BP_ProjectileBase.BP_ProjectileBase_C" _locationtransform "Undefined" 0 0)))

(event Input|AxisEvents|InputAxisLookLeft/Right
  (params (AxisValue :type Float%20%28single-precision%29))
  ;[0.3153 1 0.3519] Camera Control
  (Pawn|Input|AddControllerYawInput AxisValue))

(event Input|AxisEvents|InputAxisMoveForward/Backward
  (params (AxisValue :type Float%20%28single-precision%29))
  ;[1 0.9582 0.09561] Player Movement with my custom 'Control Rotation' function
  (bind _forwardvector (CallFunction|ControlRotation))
  (Pawn|Input|AddMovementInput _forwardvector AxisValue false))

(event Input|AxisEvents|InputAxisMoveLeft/Right
  (params (AxisValue :type Float%20%28single-precision%29))
  ;[1 0.9582 0.09561] Player Movement with my custom 'Control Rotation' function
  (bind _rightvector (CallFunction|ControlRotation))
  (Pawn|Input|AddMovementInput _rightvector AxisValue false))

(fn ConstructionScript)

(fn ControlRotation
  (bind _camera (Variables|Default|GetCamera))
  (bind _returnvalue (Transformation|GetWorldRotation _camera))
  (bind _returnvalue_2 (Math|Rotator|MakeRotator (.roll _returnvalue) (.pitch _returnvalue) (.yaw _returnvalue)))
  ;[1 1 1] Function to get the forward and right vectors for input in the Event Graph (makes for cleaner looking code)
  (return (Math|Vector|GetForwardVector _returnvalue_2) (Math|Vector|GetRightVector _returnvalue_2)))

(fn GetSceneComponentLocationIntoTransform
  (params (ObjectReference :type Scene%20Component%20Object%20Reference))
  ;[1 1 1] Function created to get the World Location and Rotation of a SceneComponent, add them together and return that as a Transform value (initially used to get the location of 'ShootDirection' arrow in order to get its location so the Player can shoot/spawn a Projectile from it)
  (bind _output_get (Variables|Default|SetObjectReference ObjectReference))
  (return (Math|Transform|MakeTransform (+ (Transformation|GetWorldLocation _output_get) (Math|Rotator|GetRotationXVector (Transformation|GetWorldRotation _output_get))) (Transformation|GetWorldRotation _output_get))))