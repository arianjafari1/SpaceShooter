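; BP_Shield is a destructible shield actor that changes color and loses health each time it is hit.
; The Hit event uses a FlipFlop to alternate the Sphere mesh between green and yellow emissive materials as visible feedback.
; A shared function applies the material, decrements and prints Health, then destroys the actor once Health reaches zero or lower.
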(event Collision|EventHit
  (params (MyComp :type Primitive%20Component%20Object%20Reference) (Other :type Actor%20Object%20Reference) (OtherComp :type Primitive%20Component%20Object%20Reference) (bSelfMoved :type Boolean) (HitLocation :type Vector :default "0, 0, 0") (HitNormal :type Vector :default "0, 0, 0") (NormalImpulse :type Vector :default "0, 0, 0") (Hit :type Hit%20Result%20Structure%20%28by%20ref%29))
  (bind _sphere (Variables|Default|GetSphere))
  ;[1 0 0.01989] Kill shield and change material to show when hit
  (Utilities|FlowControl|FlipFlop
    (:A
      (CallFunction|ToggleMaterialtoKillActor _sphere "/Game/Materials/M_GreenEmissiveMaterial_Inst.M_GreenEmissiveMaterial_Inst"))
    (:B
      (CallFunction|ToggleMaterialtoKillActor _sphere "/Game/Materials/M_YellowEmissiveMaterial_Inst.M_YellowEmissiveMaterial_Inst"))))

(fn ConstructionScript)

(fn ToggleMaterialtoKillActor
  (params (StaticMeshReference :type Static%20Mesh%20Component%20Object%20Reference) (Material :type Material%20Interface%20Object%20Reference))
  (bind _health (Variables|Default|GetHealth))
  ;[1 1 1] Function to change material when hit so the player can see the change, and destroy actor when health is 0 or lower
  (Rendering|Material|SetMaterial StaticMeshReference 0 Material)
  (bind _result (Math|Integer|DecrementInt _health)
    (:%20%20
      (Development|PrintString (Utilities|String|ToString(Integer) _result))
      (if (<= _health 0)
        (Actor|DestroyActor)))))